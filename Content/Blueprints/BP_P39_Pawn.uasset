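; BP_P39_Pawn is a player-controlled propeller aircraft pawn that flies forward constantly and fires rockets.
; Tick spins the Left and Right propellers through RotationPropeller and adds forward movement input along the actor's facing.
; Pitch and Roll axes feed controller rotation input, and the fire action spawns BP_Rocket at the Arrow component's transform.
; Manual offset and rotation movement, including Moveforworld, remains in the graph but never runs.
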(event EventTick
  (params (DeltaSeconds :type Float%20%28single-precision%29))
  ;[1 1 1] Rotate Ritht
  (CallFunction|RotationPropeller (Variables|Default|GetLeft))
  ;[1 1 1] Rotate Left
  (CallFunction|RotationPropeller (Variables|Default|GetRight))
  ;[1 1 1] Movement 이동
  (Pawn|Input|AddMovementInput (Transformation|GetActorForwardVector) 1.0 false))

(event Input|ActionEvents|InputActionfire
  (params (Key :type Key%20Structure :default "None"))
  (:Pressed
    (Game|SpawnActorfromClass "/Game/Blueprints/BP_Rocket.BP_Rocket_C" (Transformation|GetWorldTransform (Variables|Default|GetArrow)) "AdjustIfPossibleButDontSpawnIfColliding" 0 0)))

(event Input|AxisEvents|InputAxisPitch
  (params (AxisValue :type Float%20%28single-precision%29))
  ;[1 1 1] Pitch 회전
  (Pawn|Input|AddControllerPitchInput AxisValue))

(event Input|AxisEvents|InputAxisRoll
  (params (AxisValue :type Float%20%28single-precision%29))
  ;[1 1 1] Roll 회전
  (Pawn|Input|AddControllerRollInput AxisValue))

(fn ConstructionScript)

(fn RotationPropeller
  (params (Where :type Scene%20Component%20Object%20Reference))
  (Transformation|AddLocalRotation Where (Math|Rotator|MakeRotator (* (Utilities|Time|GetWorldDeltaSeconds) (Variables|속력|GetRotationSpeed)) 0.0 0.0) false false))

(fn Moveforworld
  (params (self2 :type Actor%20Object%20Reference))
  (Transformation|AddActorLocalOffset (Math|Vector|MakeVector (* (Utilities|Time|GetWorldDeltaSeconds) (Variables|속력|GetMoveSpeed)) 0.0 0.0) false false))