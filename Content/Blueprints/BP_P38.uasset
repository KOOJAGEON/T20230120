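; BP_P38 is an actor, apparently a P-38 plane, that spins two propellers and flies straight ahead.
; Each Tick it rolls the Left and Right components through a shared RotationPropeller function, then Moveforworld offsets the actor along its local X axis.
; Both motions scale RotationSpeed or MoveSpeed by world delta seconds, keeping them frame-rate independent.
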(event EventTick
  (params (DeltaSeconds :type Float%20%28single-precision%29))
  ;[1 1 1] Rotate Ritht
  (CallFunction|RotationPropeller (Variables|Default|GetLeft))
  ;[1 1 1] Rotate Left
  (CallFunction|RotationPropeller (Variables|Default|GetRight))
  ;[1 1 1] 앞으로 움직임
  (CallFunction|Moveforworld))

(fn ConstructionScript)

(fn RotationPropeller
  (params (Where :type Scene%20Component%20Object%20Reference))
  (Transformation|AddLocalRotation Where (Math|Rotator|MakeRotator (* (Utilities|Time|GetWorldDeltaSeconds) (Variables|속력|GetRotationSpeed)) 0.0 0.0) false false))

(fn Moveforworld
  (params (self2 :type Actor%20Object%20Reference))
  (Transformation|AddActorLocalOffset (Math|Vector|MakeVector (* (Utilities|Time|GetWorldDeltaSeconds) (Variables|속력|GetMoveSpeed)) 0.0 0.0) false false))